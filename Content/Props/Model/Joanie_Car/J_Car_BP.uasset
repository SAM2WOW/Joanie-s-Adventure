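; J_Car_BP is a car prop that the player character starts driving on touching its sphere trigger.
; On overlap, the car snaps onto the ThirdPersonCharacter's mesh, disables its collision and plays a lock sound.
; It switches the mesh to a looping driving animation, flags the character as InCar and raises walk speed, so character movement drives the car.
; An unconnected detach branch with a debug print never runs.
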(event OnComponentBeginOverlap(Sphere)
  (params (OverlappedComponent :type Primitive%20Component%20Object%20Reference) (OtherActor :type Actor%20Object%20Reference) (OtherComp :type Primitive%20Component%20Object%20Reference) (OtherBodyIndex :type Integer) (bFromSweep :type Boolean) (SweepResult :type Hit%20Result%20Structure%20%28by%20ref%29))
  (bind _asthird_person_character (Utilities|Casting|CastToThirdPersonCharacter OtherActor))
  (Transformation|AttachComponentToComponent (Variables|Default|GetDefaultSceneRoot) (Variables|/Script/Engine.Character|GetMesh _asthird_person_character) "None" "SnapToTarget" "SnapToTarget" "KeepWorld" true)
  (Collision|SetCollisionEnabled (Variables|Default|GetJ_Car) "NoCollision")
  (Audio|SpawnSoundatLocation "/Game/Props/Sound/Car_Lock.Car_Lock" (Transformation|GetActorLocation) "0, 0, 0" 1.0 1.0 0.0 "/Game/Props/Sound/NewSoundAttenuation.NewSoundAttenuation")
  (Components|Animation|SetAnimationMode (Variables|/Script/Engine.Character|GetMesh _asthird_person_character) "AnimationSingleNode")
  (Components|Animation|PlayAnimation (Variables|/Script/Engine.Character|GetMesh _asthird_person_character) "/Game/Props/Character/J_Driving.J_Driving" true)
  (Variables|/Game/ThirdPersonBP/Blueprints/ThirdPersonCharacter.ThirdPersonCharacter_C|SetIn%20car? _asthird_person_character true)
  (Variables|/Script/Engine.CharacterMovementComponent|SetMaxWalkSpeed (Variables|/Script/Engine.Character|GetCharacterMovement _asthird_person_character) 8e+02))

(fn ConstructionScript)