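; Rabbit prop Blueprint: an AI rabbit that wanders the level or follows the player while the player is dancing.
; After BeginPlay, a loop waits a short random delay, then checks the Dancing flag on the player's ThirdPersonCharacter.
; If dancing, AIMoveTo targets the player; otherwise it heads to a random reachable point in a very large radius.
; Both success and failure of each move restart the loop, so dancing is only rechecked between moves.
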(event EventBeginPlay
  (Utilities|FlowControl|Delay (Math|Random|RandomFloatinRange 1.0 3.0) :!label _label)
  (bind _asthird_person_character (Utilities|Casting|CastToThirdPersonCharacter (Game|GetPlayerCharacter 0)))
  (if (Variables|/Game/ThirdPersonBP/Blueprints/ThirdPersonCharacter.ThirdPersonCharacter_C|GetDancing? _asthird_person_character)
    (AI|AIMoveTo (Class|PawnMovementComponent|GetPawnOwner (Variables|Character|GetCharacterMovement)) "0, 0, 0" _asthird_person_character 5.0 false
      (:OnSuccess
        (goto _label))
      (:OnFail
        (goto _label)))
    (else
      (AI|AIMoveTo (Class|PawnMovementComponent|GetPawnOwner (Variables|Character|GetCharacterMovement)) (.RandomLocation (AI|Navigation|GetRandomReachablePointinRadius (Transformation|GetActorLocation) 1e+06 0 0)) 0 2e+01 false
        (:OnSuccess
          (goto _label))
        (:OnFail
          (goto _label))))))

(fn ConstructionScript)