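; Gulab is an AI pawn, apparently a dog, that follows the player and makes a sound on reaching them.
; A looping one-second timer started at BeginPlay calls Walk, which issues an AI MoveTo toward the player pawn.
; A successful move fires a DoOnce that spawns the attenuated Dog sound with random volume and pitch.
; The DoOnce resets when the MoveTo result checked after issuing the move equals Aborted.
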(event Custom|Walk
  (bind _returnvalue (Game|Player|GetPlayerPawn 0))
  (bind _movementresult (AI|AIMoveTo self (Transformation|GetActorLocation _returnvalue) _returnvalue 1e+02 false)
    (:then
      (if (Utilities|Enum|Equal(Enum) _movementresult "Aborted")
        (goto _label Reset)))
    (:OnSuccess
      (Utilities|FlowControl|DoOnce false :!label _label
        (:Completed
          (Audio|SpawnSoundatLocation "/Game/Props/Sound/Dog.Dog" (Transformation|GetActorLocation) "0, 0, 0" (Math|Random|RandomFloatinRange 0.5 0.8) (Math|Random|RandomFloatinRange 0.9 1.1) 0.0 "/Game/Props/Sound/NewSoundAttenuation.NewSoundAttenuation" 0))))))

(event EventBeginPlay
  (Utilities|Time|SetTimerbyFunctionName 0 "Walk" 1.0 true))

(fn ConstructionScript)