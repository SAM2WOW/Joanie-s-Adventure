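; Ladybug collectible pawn that wanders the navmesh and is caught when the third-person character overlaps its sphere.
; On begin play it loops AI moves to random reachable points, pausing up to a second after each success or failure.
; A catch fires once, increments the player's ladybug count, calls Pickup and plays a sound.
; It then spawns a replacement at a random navigable point around the player and destroys itself.
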(event OnComponentBeginOverlap(Sphere)
  (params (OverlappedComponent :type Primitive%20Component%20Object%20Reference) (OtherActor :type Actor%20Object%20Reference) (OtherComp :type Primitive%20Component%20Object%20Reference) (OtherBodyIndex :type Integer) (bFromSweep :type Boolean) (SweepResult :type Hit%20Result%20Structure%20%28by%20ref%29))
  (bind _asthird_person_character (Utilities|Casting|CastToThirdPersonCharacter OtherActor))
  (Utilities|FlowControl|DoOnce false
    (:Completed
      (Variables|/Game/ThirdPersonBP/Blueprints/ThirdPersonCharacter.ThirdPersonCharacter_C|SetLadybug _asthird_person_character (+ (Variables|/Game/ThirdPersonBP/Blueprints/ThirdPersonCharacter.ThirdPersonCharacter_C|GetLadybug _asthird_person_character) 1))
      (Default|Pickup _asthird_person_character)
      (Audio|PlaySoundatLocation "/Game/Props/Sound/Catch_Bug.Catch_Bug" (Transformation|GetActorLocation) "0, 0, 0" 1.0 1.0 0.0 "/Game/Props/Sound/NewSoundAttenuation.NewSoundAttenuation" 0 0)
      (Game|SpawnActorfromClass "Ladybug_BP_C" (Math|Transform|MakeTransform (.RandomLocation (Class|NavigationSystemV1|GetRandomPointinNavigableRadius (Transformation|GetActorLocation (Game|GetPlayerCharacter 0)) 1e+05 0 0))) "AdjustIfPossibleButAlwaysSpawn" 0 0)
      (Actor|DestroyActor))))

(event EventBeginPlay
  (AI|AIMoveTo (Class|PawnMovementComponent|GetPawnOwner (Variables|Character|GetCharacterMovement)) (.RandomLocation (AI|Navigation|GetRandomReachablePointinRadius (Transformation|GetActorLocation) 1e+06 0 0)) 0 5.0 false :!label _label
    (:OnSuccess
      _)
    (:OnFail
      _))
  (Utilities|FlowControl|Delay (Math|Random|RandomFloatinRange 0.0 1.0))
  (goto _label))

(fn ConstructionScript)